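; BP_DoorExample is an example door Blueprint that drives a movement sound from how fast the door moves.
; It listens to the DoorMovedDelegate of its DoorMovement component, which reports a movement delta.
; When the delta's magnitude passes a small threshold, the Audio component starts or resumes, with volume scaled and clamped from that magnitude.
; Below the threshold the sound pauses, so later movement can resume it.
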(event DoorMovedDelegate(DoorMovement)
  (params (Delta :type Float%20%28single-precision%29))
  (bind _returnvalue (Math|Float|Absolute(Float) Delta))
  (bind _audio (Variables|Default|GetAudio))
  (if (>= _returnvalue 0.001)
    (if (Audio|Components|Audio|IsPlaying _audio)
      (Class|AudioComponent|SetPaused _audio false)
      (else
        (Audio|Components|Audio|Play _audio 0.0)))
    (Audio|Components|Audio|SetVolumeMultiplier _audio (Math|Float|Clamp(Float) (* _returnvalue 5e+01)) :!class /Script/Engine.AudioComponent)
    (else
      (Class|AudioComponent|SetPaused _audio true))))

(event EventBeginPlay)

(event Collision|EventActorBeginOverlap
  (params (OtherActor :type Actor%20Object%20Reference)))

(event EventTick
  (params (DeltaSeconds :type Float%20%28single-precision%29)))

(fn ConstructionScript)